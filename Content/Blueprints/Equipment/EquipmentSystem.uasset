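; Equipment component that spawns and tracks an owner's equipped items, keyed by slot type.
; Equip spawns the item's actor class at the owner, registers it in the Items map, initializes it and briefly draws its name as debug text.
; Fire forwards a direction to the item in one fixed slot, while SetAimDirection passes aim to every equipped item.
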(event EventEquip
  (params (ItemStructure :type Item%20Structure%20Structure))
  (bind (_name _itemslottype _staticmesh _actorclass) (Utilities|Struct|BreakItemStructure ItemStructure))
  (bind _returnvalue (Components|GetOwner))
  (bind _returnvalue_2 (Game|SpawnActorfromClass _actorclass (Transformation|GetActorTransform _returnvalue) "AlwaysSpawn" _returnvalue 0))
  (bind _asitem (Utilities|Casting|CastToItem _returnvalue_2))
  (Utilities|Map|Add (Variables|Default|Getitems) _itemslottype _asitem)
  (Default|Equip _asitem ItemStructure)
  (Rendering|Debug|DrawDebugString (Transformation|GetActorLocation (Components|GetOwner)) (Utilities|String|ToString(Text) _name) 0 "(R=1.000000,G=0.032634,B=0.000000,A=1.000000)" 2.0))

(event EventFire
  (params (direction :type Vector :default "0, 0, 0"))
  (bind _items (Variables|Default|Getitems))
  (bind (_value _returnvalue) (Utilities|Map|Find _items "NewEnumerator0"))
  (if _returnvalue
    (Default|Fire _value direction)))

(event EventSetAimDirection
  (params (direction :type Vector :default "0, 0, 0"))
  (bind _keys (Utilities|Map|Keys (Variables|Default|Getitems)))
  (for _array_element _keys
    (Default|SetAimDirection (.Value (Utilities|Map|Find (Variables|Default|Getitems) _array_element)) direction)))