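; Pickup actor that gives a randomly chosen item to whoever overlaps it.
; On BeginPlay, GetRandomItem picks a random row from ItemsDataTable and stores it as the item structure.
; When its sphere is overlapped, it looks for an EquipmentSystem component on the overlapping actor's instigator controller, passes the item via EquipMessage, then destroys itself.
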(event OnComponentBeginOverlap(Sphere)
  (params (OverlappedComponent :type Primitive%20Component%20Object%20Reference) (OtherActor :type Actor%20Object%20Reference) (OtherComp :type Primitive%20Component%20Object%20Reference) (OtherBodyIndex :type Integer) (bFromSweep :type Boolean) (SweepResult :type Hit%20Result%20Structure%20%28by%20ref%29))
  (bind _returnvalue (Game|GetInstigatorController OtherActor))
  (bind _returnvalue_2 (Actor|GetComponentbyClass _returnvalue "/Game/Blueprints/Equipment/EquipmentSystem.EquipmentSystem_C"))
  (Utilities|IsValid _returnvalue_2
    (:Is%20Valid
      (Class|Equipment|Equip(Message) _returnvalue_2 (Variables|Default|GetItemStructure))
      (Actor|DestroyActor))))

(event EventBeginPlay
  (bind _out_row (CallFunction|GetRandomItem))
  (Variables|Default|SetItemStructure _out_row))

(fn ConstructionScript)

(fn GetRandomItem
  (bind _outrownames (DataTable|GetDataTableRowNames "/Game/Blueprints/Equipment/ItemsDataTable.ItemsDataTable"))
  (bind _returnvalue (Utilities|GetDataTableRow "/Game/Blueprints/Equipment/ItemsDataTable.ItemsDataTable" (Utilities|Array|Get(acopy) _outrownames (Math|Random|RandomIntegerinRange 0 (- (Utilities|Array|Length _outrownames) 1))))
    (:then
      (return _returnvalue))))