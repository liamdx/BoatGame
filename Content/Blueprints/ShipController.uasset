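; Player controller for a ship in a boat game, handling twin-stick movement and aiming, firing, health and player number.
; Movement follows world axes, while look and turn axes set a flat AimDirection, drawn as a debug arrow and passed to EquipmentSystem to fire.
; Keys and gamepad special buttons spawn or despawn the player through BoatGameMode.
; DoDamage despawns through Die, but its death check subtracts damage a second time.
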(event EventBeginPlay)

(event Input|ActionEvents|InputActionFire
  (params (Key :type Key%20Structure))
  (bind _returnvalue (Actor|GetComponentbyClass "/Game/Blueprints/Equipment/EquipmentSystem.EquipmentSystem_C"))
  (bind _aimdirection (Variables|Default|GetaimDirection))
  (:Pressed
    (Utilities|IsValid _returnvalue
      (:Is%20Valid
        (Class|Equipment|Fire(Message) _returnvalue _aimdirection (+ (Transformation|GetWorldLocation (Variables|/Script/Engine.Actor|GetRootComponent (Pawn|GetControlledPawn))) (* _aimdirection 5e+02)) self)))))

(event Input|AxisEvents|InputAxisMoveForward
  (params (AxisValue :type Float%20%28single-precision%29))
  (bind _returnvalue (Pawn|GetControlledPawn))
  (Utilities|IsValid _returnvalue
    (:Is%20Valid
      (Pawn|Input|AddMovementInput _returnvalue "1.000000, 0, 0" AxisValue false))))

(event Input|AxisEvents|InputAxisMoveRight
  (params (AxisValue :type Float%20%28single-precision%29))
  (bind _returnvalue (Pawn|GetControlledPawn))
  (Utilities|IsValid _returnvalue
    (:Is%20Valid
      (Pawn|Input|AddMovementInput _returnvalue "0.000000,1.000000, 0" AxisValue false))))

(event Input|AxisEvents|InputAxisLookUpRate
  (params (AxisValue :type Float%20%28single-precision%29))
  (bind _returnvalue (Pawn|GetControlledPawn))
  (bind _returnvalue_2 (Transformation|GetActorLocation _returnvalue))
  (Utilities|IsValid _returnvalue
    (:Is%20Valid
      (Utilities|FlowControl|Sequence
        (:then_0
          (Variables|Default|SetaimDirection (Math|Vector|MakeVector (* 1.0 AxisValue) (.y (Variables|Default|GetaimDirection)) 0.0)))
        (:then_1
          (Rendering|Debug|DrawDebugArrow _returnvalue_2 (+ _returnvalue_2 (* (Variables|Default|GetaimDirection) 5e+02)) 1e+02 "(R=0.560000,G=0.000000,B=0.000000,A=1.000000)" 0.0 5e+01))))))

(event Input|AxisEvents|InputAxisTurnRate
  (params (AxisValue :type Float%20%28single-precision%29))
  (bind _returnvalue (Pawn|GetControlledPawn))
  (bind _returnvalue_2 (Transformation|GetActorLocation _returnvalue))
  (Utilities|IsValid _returnvalue
    (:Is%20Valid
      (Utilities|FlowControl|Sequence
        (:then_0
          (Variables|Default|SetaimDirection (Math|Vector|MakeVector (.x (Variables|Default|GetaimDirection)) (* 1.0 AxisValue) 0.0)))
        (:then_1
          (Rendering|Debug|DrawDebugArrow _returnvalue_2 (+ _returnvalue_2 (* (Variables|Default|GetaimDirection) 5e+02)) 1e+02 "(R=0.560000,G=0.000000,B=0.000000,A=1.000000)" 0.0 5e+01))))))

(event Input|GamepadEvents|GamepadSpecialLeft
  (params (Key :type Key%20Structure))
  (:Pressed
    (bind _asboat_game_mode (Utilities|Casting|CastToBoatGameMode (Game|GetGameMode)))
    (Default|DespawnCharacter _asboat_game_mode self)))

(event Input|GamepadEvents|GamepadSpecialRight
  (params (Key :type Key%20Structure))
  (:Pressed
    (bind _asboat_game_mode (Utilities|Casting|CastToBoatGameMode (Game|GetGameMode)))
    (Default|SpawnCharacter _asboat_game_mode self)))

(event Input|KeyboardEvents|J
  (params (Key :type Key%20Structure))
  (:Pressed
    (bind _asboat_game_mode (Utilities|Casting|CastToBoatGameMode (Game|GetGameMode)))
    (Default|SpawnCharacter _asboat_game_mode self)))

(event Input|KeyboardEvents|K
  (params (Key :type Key%20Structure))
  (:Pressed
    (bind _asboat_game_mode (Utilities|Casting|CastToBoatGameMode (Game|GetGameMode)))
    (Default|DespawnCharacter _asboat_game_mode self)))

(fn ConstructionScript
  (bind _asboat_game_mode (Utilities|Casting|CastToBoatGameMode (Game|GetGameMode)))
  (Variables|Default|SetgameMode _asboat_game_mode)
  (Default|SetItemControllers (Variables|Default|GetEquipmentSystem) self))

(fn GetAimDirection
  (return (Variables|Default|GetaimDirection)))

(fn DoDamage
  (params (Damage :type Integer))
  (Variables|Default|Sethealth (- (Variables|Default|Gethealth) Damage))
  (if (<= (- (Variables|Default|Gethealth) Damage) 0)
    (CallFunction|Die)))

(fn Die
  (Default|DespawnCharacter (Variables|Default|GetgameMode) self))

(fn SetPlayerNo
  (params (playerNo :type Integer))
  (Variables|Default|SetplayerNumber playerNo))

(fn GetPlayerNo
  (return (Variables|Default|GetplayerNumber)))