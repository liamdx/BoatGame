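; Player-controlled ship pawn that floats through a buoyancy function on its static mesh and is driven by physics thrusters.
; Each tick, left-stick Y sets forward or backpedal thrust past a deadzone.
; Left-stick X picks diagonal thruster pairs scaled by a stick-to-heading dot product, but a zero multiplier currently disables their thrust.
; Debug lines and printed text show that direction test.
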(event EventBeginPlay
  ;[1 1 1] Set thruster values
  (Input|EnableInput (Game|GetPlayerController 0))
  (Components|Activation|SetActive (Variables|Default|GetFrontRightThruster) true false))

(event EventTick
  (params (DeltaSeconds :type Float%20%28single-precision%29))
  (bind _returnvalue (Transformation|GetActorLocation))
  (bind _staticmesh (Variables|Default|GetStaticMesh))
  (bind _returnvalue_2 (Math|Vector|GetForwardVector _staticmesh))
  (bind _returnvalue_3 (* _returnvalue (Math|Vector|MakeVector (.x _returnvalue_2) (.y _returnvalue_2) (.z _returnvalue_2))))
  ;[1 1 1] Uncategorized
  (CallFunction|BuoyancyFunction (Variables|Default|GetStaticMesh) 4e+02 "ObjectTypeQuery7")
  (Utilities|FlowControl|Sequence
    (:then_1
      ;[1 1 1] Debug Direction Testing
      (Variables|Default|SetTargetAngleDot (Math|Vector|DotProduct (Math|Vector|Normalize (* _returnvalue (Math|Vector|MakeVector (* (stale Input|GamepadEvents|GamepadLeftX AxisValue) 4e+02) (* (stale Input|GamepadEvents|GamepadLeftY AxisValue) -4e+02) 0.0))) (Math|Vector|Normalize _returnvalue_3)))
      (Rendering|Debug|DrawDebugLine _returnvalue (* _returnvalue (Math|Vector|MakeVector (* (stale Input|GamepadEvents|GamepadLeftX AxisValue) 4e+02) (* (stale Input|GamepadEvents|GamepadLeftY AxisValue) -4e+02) 0.0)) "(R=1.000000,G=0.000000,B=0.833858,A=1.000000)" 0.05 5e+01)
      (Rendering|Debug|DrawDebugLine _returnvalue (* _returnvalue_3 4e+02) "(R=0.013568,G=0.000000,B=1.000000,A=1.000000)" 0.05 5e+01)
      (Development|PrintText (Utilities|Text|ToText(Float) (Math|Float|NormalizetoRange (Math|Vector|DotProduct (Math|Vector|Normalize (* _returnvalue (Math|Vector|MakeVector (* (stale Input|GamepadEvents|GamepadLeftX AxisValue) 4e+02) (* (stale Input|GamepadEvents|GamepadLeftY AxisValue) -4e+02) 0.0))) (Math|Vector|Normalize _returnvalue_3)) -1.0 1.0) "HalfToEven" false true 1 324 5 10))
      (Utilities|FlowControl|Sequence
        (:then_0
          (if (>= (Variables|Default|GetGamepadLeftThumbX) 0.0)
            (Variables|Default|SetRightThrustStrength (* (* (* (Math|Float|Absolute(Float) (Variables|Default|GetGamepadLeftThumbX)) 2e+04) (- 1.0 (Math|Float|Absolute(Float) (Variables|Default|GetTargetAngleDot)))) 0.0))
            (Variables|Default|SetLeftThrustStrength 0.0)
            (else
              (Variables|Default|SetRightThrustStrength 0.0)
              (Variables|Default|SetLeftThrustStrength (* (* (* (Math|Float|Absolute(Float) (Variables|Default|GetGamepadLeftThumbX)) 2e+04) (- 1.0 (Math|Float|Absolute(Float) (Variables|Default|GetTargetAngleDot)))) 0.0)))))
        (:then_1
          (if (>= (Variables|Default|GetGamepadLeftThumbY) 0.0)
            (Variables|Default|SetForwardThrustStrength (Variables|Default|GetangleMultiplier))
            (Variables|Default|SetBackpedalThrustStrength 0.0)
            (else
              (Variables|Default|SetForwardThrustStrength 0.0)
              (Variables|Default|SetBackpedalThrustStrength (Variables|Default|GetangleMultiplier)))))
        (:then_2
          (if (>= (Math|Float|Absolute(Float) (Variables|Default|GetGamepadLeftThumbY)) (Variables|Default|GetboatDotDeatzone))
            (Variables|Default|SetangleMultiplier (* (Math|Float|Absolute(Float) (Variables|Default|GetGamepadLeftThumbY)) 1e+06))
            (else
              (Variables|Default|SetangleMultiplier 0.0))))
        (:then_3
          ;[1 1 1] Set thruster values
          (Variables|/Script/Engine.PhysicsThrusterComponent|SetThrustStrength (Variables|Default|GetBackpedalThruster) (Variables|Default|GetBackpedalThrustStrength))
          ;;[1 1 1] left
          (Variables|/Script/Engine.PhysicsThrusterComponent|SetThrustStrength (Variables|Default|GetRearLeftThruster) (Variables|Default|GetLeftThrustStrength))
          (Variables|/Script/Engine.PhysicsThrusterComponent|SetThrustStrength (Variables|Default|GetFrontRightThruster) (Variables|Default|GetLeftThrustStrength))
          ;;[1 1 1] right
          (Variables|/Script/Engine.PhysicsThrusterComponent|SetThrustStrength (Variables|Default|GetRearRightThruster) (Variables|Default|GetRightThrustStrength))
          (Variables|/Script/Engine.PhysicsThrusterComponent|SetThrustStrength (Variables|Default|GetFrontLeftThruster) (Variables|Default|GetRightThrustStrength))
          (Variables|/Script/Engine.PhysicsThrusterComponent|SetThrustStrength (Variables|Default|GetForwardThruster) (Variables|Default|GetForwardThrustStrength)))))
    (:then_2
      (Variables|Default|SetGamepadLeftThumbX (stale Input|GamepadEvents|GamepadLeftX AxisValue))
      (Variables|Default|SetGamepadLeftThumbY (stale Input|GamepadEvents|GamepadLeftY AxisValue)))))

(event Input|GamepadEvents|GamepadLeftX
  (params (AxisValue :type Float%20%28single-precision%29))
  ;[1 1 1] Uncategorized
)

(event Input|GamepadEvents|GamepadLeftY
  (params (AxisValue :type Float%20%28single-precision%29))
  ;[1 1 1] Uncategorized
)

(fn ConstructionScript)