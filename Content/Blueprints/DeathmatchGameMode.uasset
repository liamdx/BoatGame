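; Deathmatch game mode that sets up local multiplayer pawns and a shared camera view at BeginPlay.
; SpawnCamera, marked temporary, takes the first existing CameraActor rather than spawning one.
; For each tagged "shipStart" PlayerStart, SpawnPlayers creates missing local players, then re-loops all collected starts to spawn and possess TesticlePawns, so earlier starts repeat.
; PossessPawns then has controller 0 possess every pawn in turn and view through that camera.
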(event EventBeginPlay
  (bind _camera (CallFunction|SpawnCamera))
  (Variables|Default|SetCamera _camera)
  (CallFunction|SpawnPlayers)
  (CallFunction|PossessPawns))

(event EventTick
  (params (DeltaSeconds :type Float%20%28single-precision%29)))

(fn ConstructionScript)

(fn SpawnPlayers
  (bind _outactors (Actor|GetAllActorswithTag "shipStart"))
  (Development|PrintString (Utilities|String|ToString(Integer) (Utilities|Array|Length _outactors)))
  (for _array_element _outactors
    (bind _asplayer_start (Utilities|Casting|CastToPlayerStart _array_element))
    (Utilities|Array|Add (LocalVariables|GetplayerStarts) _asplayer_start)
    (for _index (range 0 (- (Variables|Default|GetmaxPlayers) 1))
      (Utilities|IsValid (Game|GetPlayerController _index)
        (:Is%20Not%20Valid
          (Class|GameplayStatics|CreatePlayer _index))))
    (for _index_2 (range 0 (- (Utilities|Array|Length (LocalVariables|GetplayerStarts)) 1))
      (bind _returnvalue (Game|SpawnActorfromClass "/Game/Blueprints/TesticlePawn.TesticlePawn_C" (Transformation|GetActorTransform (Utilities|Array|Get(acopy) (LocalVariables|GetplayerStarts) _index_2)) "Undefined" 0 0))
      (Pawn|Possess (Game|GetPlayerController _index_2) _returnvalue))))

(fn SpawnCamera
  (bind _outactors (Actor|GetAllActorsOfClass "/Script/Engine.CameraActor")) ; Temp
  (return (Utilities|Array|Get(acopy) _outactors)))

(fn PossessPawns
  (bind _returnvalue (Game|GetPlayerController 0))
  (bind _outactors (Actor|GetAllActorsOfClass "/Game/Blueprints/TesticlePawn.TesticlePawn_C"))
  (for _array_element _outactors
    (Pawn|Possess _returnvalue _array_element)
    (Game|Player|SetViewTargetwithBlend _returnvalue (Variables|Default|GetCamera) 0.0 "VTBlend_Linear" 0.0 false)))