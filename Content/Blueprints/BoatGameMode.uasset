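; Game mode for a multiplayer boat game that creates local players and handles spawning and despawning their boats.
; BeginPlay caches all PlayerStarts, then creates players up to MaxPlayers, storing and numbering each ShipController.
; SpawnCharacter acts only when the controller already has a pawn, replacing it with a possessed Boat at a random cached start and calling CallPlayerJoined.
; DespawnCharacter unpossesses before calling destroy on the controlled pawn.
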(event Custom|SpawnCharacter
  (params (PlayerController :type Ship%20Controller%20Object%20Reference))
  (bind _returnvalue (Pawn|GetControlledPawn PlayerController))
  (bind _spawns (Variables|Default|GetSpawns))
  (Utilities|IsValid _returnvalue
    (:Is%20Valid
      (Actor|DestroyActor _returnvalue)
      (bind _returnvalue_2 (Game|SpawnActorfromClass "/Game/Blueprints/Boat.Boat_C" (Math|Transform|MakeTransform (Math|Transform|TransformLocation (Transformation|GetActorTransform (Utilities|Array|Get(acopy) _spawns (Math|Random|RandomInteger (- (Utilities|Array|Length _spawns) 1)))) "0, 0, 0")) "Undefined" 0 0))
      (Default|SetBoatController _returnvalue_2 PlayerController)
      (Default|CallPlayerJoined PlayerController _returnvalue_2)
      (Pawn|Possess PlayerController _returnvalue_2))))

(event Custom|DespawnCharacter
  (params (PlayerController :type Ship%20Controller%20Object%20Reference))
  (Pawn|UnPossess PlayerController)
  (Actor|DestroyActor (Pawn|GetControlledPawn PlayerController)))

(event EventBeginPlay
  (bind _outactors (Actor|GetAllActorsOfClass "/Script/Engine.PlayerStart"))
  (Variables|Default|SetSpawns _outactors)
  (for _index (range 0 (- (Variables|Default|GetmaxPlayers) 1))
    (bind _returnvalue (Class|GameplayStatics|CreatePlayer _index))
    (bind _asship_controller (Utilities|Casting|CastToShipController _returnvalue)
      (:then
        (Development|PrintString "Cast from player to ship controller succeeded")
        (bind _returnvalue_2 (Utilities|Array|Add (Variables|Default|GetPlayers) _asship_controller))
        (Default|SetPlayerNo _asship_controller _returnvalue_2))
      (:CastFailed
        (Development|PrintString "Cast from player to ship controller failed")))))

(event EventTick
  (params (DeltaSeconds :type Float%20%28single-precision%29)))

(fn ConstructionScript)