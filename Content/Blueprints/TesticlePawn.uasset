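; TesticlePawn is a physics-driven pawn whose static mesh floats and moves by movement input.
; Each Tick calls BuoyancyFunction on the mesh with a custom object channel, then HandleMovement.
; HandleMovement consumes the input vector and, when non-zero, applies a delta-scaled force as an acceleration change, so mass is ignored.
; It also eases the actor's rotation toward the input direction with RInterpTo.
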(event EventBeginPlay)

(event Collision|EventActorBeginOverlap
  (params (OtherActor :type Actor%20Object%20Reference)))

(event EventTick
  (params (DeltaSeconds :type Float%20%28single-precision%29))
  (CallFunction|BuoyancyFunction (Variables|Default|GetStaticMesh) 4e+02 "ObjectTypeQuery7")
  (CallFunction|HandleMovement))

(fn ConstructionScript)

(fn HandleMovement
  (bind _staticmesh (Variables|Default|GetStaticMesh))
  (bind _returnvalue (Class|Pawn|ConsumeMovementInputVector))
  (bind _output_get (LocalVariables|SetmovementInputVector _returnvalue))
  (if (> (Math|Vector|VectorLength _output_get) 0.0)
    (Physics|AddForce _staticmesh (* _output_get (* (Variables|Default|GetmovementSpeed) (Utilities|Time|GetWorldDeltaSeconds) 1e+02)) "None" true)
    (Transformation|SetActorRotation (Math|Interpolation|RInterpTo (Transformation|GetWorldRotation _staticmesh) (Math|Rotator|MakeRotfromX (LocalVariables|GetmovementInputVector)) (Utilities|Time|GetWorldDeltaSeconds) 1.0))))