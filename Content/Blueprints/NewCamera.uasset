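; NewCamera is a camera actor that follows all Boat actors in the level as a group.
; Each tick it finds every Boat, averages their locations and moves its Box component to a fixed offset behind and above that point.
; It also eases the Box's pitch slowly toward the group centre with RInterpTo.
; An unconnected older version moves the Camera component directly and includes an unused bounds-based zoom height.
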(event EventBeginPlay)

(event EventTick
  (params (DeltaSeconds :type Float%20%28single-precision%29))
  (bind _box (Variables|Default|GetBox))
  (bind _outactors (Actor|GetAllActorsOfClass "/Game/Blueprints/Boat.Boat_C"))
  (bind _returnvalue (Class|GameplayStatics|GetActorArrayAverageLocation _outactors))
  (Transformation|SetWorldRotation _box (Math|Rotator|MakeRotator 0.0 (.pitch (Math|Interpolation|RInterpTo (Transformation|GetWorldRotation _box) (Math|Rotator|FindLookatRotation (Transformation|GetWorldLocation _box) _returnvalue) DeltaSeconds 0.05)) 0.0) false false)
  (Transformation|SetWorldLocation _box (+ _returnvalue "-3000.000000, 0,5000.000000") false false))

(fn ConstructionScript)